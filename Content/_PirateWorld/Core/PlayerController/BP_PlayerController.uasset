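; BP_PlayerController maps player input to the controlled pawn in the pirate world game.
; Movement axes push the pawn along the camera manager's forward and right vectors, making movement camera-relative, while look axes add pitch and yaw input.
; Jump and primary attack presses are forwarded to the pawn by casting it to BP_CharacterBase.
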(event EventBeginPlay)

(event EventTick
  (params (DeltaSeconds :type Float%20%28single-precision%29)))

(event Input|ActionEvents|InputActionJump
  (params (Key :type Key%20Structure :default "None"))
  (:Pressed
    (Character|Jump (.AsBP%20Character%20Base (Utilities|Casting|CastToBP_CharacterBase (Pawn|GetControlledPawn))))))

(event Input|ActionEvents|InputActionPrimaryAttack
  (params (Key :type Key%20Structure :default "None"))
  (:Pressed
    (Default|PrimaryAttack (.AsBP%20Character%20Base (Utilities|Casting|CastToBP_CharacterBase (Pawn|GetControlledPawn))))))

(event Input|AxisEvents|InputAxisMoveForward
  (params (AxisValue :type Float%20%28single-precision%29))
  (Pawn|Input|AddMovementInput (Pawn|GetControlledPawn) (Math|Vector|GetForwardVector (Camera|GetCameraRotation (Variables|Default|GetPlayerCameraManager))) AxisValue false))

(event Input|AxisEvents|InputAxisMoveRight
  (params (AxisValue :type Float%20%28single-precision%29))
  (Pawn|Input|AddMovementInput (Pawn|GetControlledPawn) (Math|Vector|GetRightVector (Camera|GetCameraRotation (Variables|Default|GetPlayerCameraManager))) AxisValue false))

(event Input|AxisEvents|InputAxisLookUp
  (params (AxisValue :type Float%20%28single-precision%29))
  (Class|PlayerController|AddPitchInput AxisValue))

(event Input|AxisEvents|InputAxisTurn
  (params (AxisValue :type Float%20%28single-precision%29))
  (Class|PlayerController|AddYawInput AxisValue))

(fn ConstructionScript)