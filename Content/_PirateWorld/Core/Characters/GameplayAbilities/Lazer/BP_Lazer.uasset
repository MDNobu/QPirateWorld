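; Laser beam actor for a gameplay ability that deals repeated damage to hostile characters overlapping its LazerEndDetector.
; Tick stretches the skeletal beam by feeding the detector's distance, minus the initial socket length, to ABP_LazerBeam as an end offset.
; Overlap events maintain the enemy list, filtered by hostility to the instigator.
; A looping timer sends that list as target data in a gameplay event to the instigator, delegating damage.
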(event OnComponentBeginOverlap(LazerEndDetector)
  (params (OverlappedComponent :type Primitive%20Component%20Object%20Reference) (OtherActor :type Actor%20Object%20Reference) (OtherComp :type Primitive%20Component%20Object%20Reference) (OtherBodyIndex :type Integer) (bFromSweep :type Boolean) (SweepResult :type Hit%20Result%20Structure%20%28by%20ref%29))
  (bind _asbp_character_base (Utilities|Casting|CastToBP_CharacterBase OtherActor))
  (if (Class|QCharacterBase|IsHostile _asbp_character_base (.AsBP%20Character%20Base (Utilities|Casting|CastToBP_CharacterBase (Game|GetInstigator))))
    (Utilities|Array|AddUnique (Variables|Default|GetOverlappingEnemies) _asbp_character_base)))

(event OnComponentEndOverlap(LazerEndDetector)
  (params (OverlappedComponent :type Primitive%20Component%20Object%20Reference) (OtherActor :type Actor%20Object%20Reference) (OtherComp :type Primitive%20Component%20Object%20Reference) (OtherBodyIndex :type Integer))
  (bind _asbp_character_base (Utilities|Casting|CastToBP_CharacterBase OtherActor))
  (if (Class|QCharacterBase|IsHostile _asbp_character_base (.AsBP%20Character%20Base (Utilities|Casting|CastToBP_CharacterBase (Game|GetInstigator))))
    (Utilities|Array|RemoveItem (Variables|Default|GetOverlappingEnemies) _asbp_character_base)))

(event Custom|ContinousDamageEnemy
  (bind _returnvalue (Game|GetInstigator))
  (bind _overlappingenemies (Variables|Default|GetOverlappingEnemies))
  (if (> (Utilities|Array|Length _overlappingenemies) 0)
    _
    (else
      _))
  (Ability|SendGameplayEventtoActor _returnvalue "(TagName=\"skill.lazer.dealDamage\")" (Utilities|Struct|MakeGameplayEventData "(TagName=\"\")" _returnvalue 0 0 0 "()" "(GameplayTags=)" "(GameplayTags=)" 0.0 (Ability|TargetData|AbilityTargetDatafromActorArray _overlappingenemies))))

(event EventBeginPlay
  (Utilities|FlowControl|Sequence
    (:then_0
      (bind _asabp_lazer_beam (Utilities|Casting|CastToABP_LazerBeam (Components|SkeletalMesh|GetAnimInstance (Variables|Default|GetSkeletalMesh))))
      (Variables|Default|SetAPB_LazerBeam _asabp_lazer_beam))
    (:then_1
      (Variables|Default|SetInitBeamLength (Math|Vector|VectorLength (- (Transformation|GetSocketLocation (Variables|Default|GetSkeletalMesh) "end") (Transformation|GetActorLocation)))))
    (:then_2
      (Utilities|Time|SetTimerbyEvent (delegate Custom|ContinousDamageEnemy) 0.3 true))))

(event EventTick
  (params (DeltaSeconds :type Float%20%28single-precision%29))
  (Variables|/Game/_PirateWorld/Core/Characters/GameplayAbilities/Lazer/LazerAssets/ABP_LazerBeam.ABP_LazerBeam_C|SetBeamEndOffset (Variables|Default|GetAPB_LazerBeam) (Math|Vector|MakeVector (- (Math|Vector|VectorLength (- (Transformation|GetWorldLocation (Variables|Default|GetLazerEndDetector)) (Transformation|GetActorLocation))) (Variables|Default|GetInitBeamLength)) 0.0 0.0)))

(fn ConstructionScript)