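; Player gameplay ability that plays a casting montage and, after a short delay, spawns a laser actor attached to the character mesh's LazerSocket.
; Each Skill.lazer.dealDamage event applies damage to its target data, then pushes and stuns those characters along the beam, provided the cost resource suffices.
; Insufficient resource ends the ability; ending destroys the laser and removes the cost effect.
; Control-rotation mode is set true on both spawn and end.
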(event Ability|EventActivateAbility
  (Ability|CommitAbility)
  (CallFunction|StartCooldown)
  (|PlayMontageandWaitProxy "None" "/Game/_PirateWorld/Core/Characters/Animations/AM_Shinbi_CastLazer.AM_Shinbi_CastLazer" 1.0 "None" true 1.0 0.0
    (:then
      (Utilities|FlowControl|Delay 0.3)
      (bind _bp_character_player (CallFunction|GetPlayerCharacterandController))
      (Utilities|IsValid _bp_character_player
        (:Is%20Valid
          (bind _spawnedactor (|SpawnActor :Class "/Game/_PirateWorld/Core/Characters/GameplayAbilities/Lazer/BP_Lazer.BP_Lazer_C" :Instigator _bp_character_player)
            (:then
              (Variables|Default|SetLazerActor _spawnedactor)
              (Transformation|AttachComponentToComponent _spawnedactor (Variables|/Script/Engine.Character|GetMesh _bp_character_player) "LazerSocket" "SnapToTarget" "SnapToTarget" "KeepRelative" true)
              (Default|SetUseControlRotatioinMode _bp_character_player true)
              (bind _payload (Ability|Tasks|WaitGameplayEvent "(TagName=\"skill.lazer.dealDamage\")" 0)
                (:EventReceived
                  (bind _costenough (CallFunction|IsCostResourceEnough))
                  (if _costenough
                    (GameplayEffects|ApplyGameplayEffectToTarget (.TargetData (Utilities|Struct|BreakGameplayEventData _payload)) "/Game/_PirateWorld/Core/Characters/GameplayAbilities/Lazer/BP_GE_Lazer_DealDamage.BP_GE_Lazer_DealDamage_C" 1 1)
                    (for _array_element (Ability|TargetData|GetAllActorsfromTargetData (.TargetData (Utilities|Struct|BreakGameplayEventData _payload)))
                      (bind _asbp_character_base (Utilities|Casting|CastToBP_CharacterBase _array_element))
                      (Default|PushandStunCharacter _asbp_character_base (Math|Vector|Normalize (- (Transformation|GetWorldLocation (Variables|/Game/_PirateWorld/Core/Characters/GameplayAbilities/Lazer/BP_Lazer.BP_Lazer_C|GetLazerEndDetector (.AsBP%20Lazer (Utilities|Casting|CastToBP_Lazer (Variables|Default|GetLazerActor))))) (Transformation|GetActorLocation (.AsBP%20Lazer (Utilities|Casting|CastToBP_Lazer (Variables|Default|GetLazerActor)))))) 5e+02 0.3 "/Game/_PirateWorld/Core/Characters/Animations/AM_HitStun.AM_HitStun"))
                    (else
                      (Ability|EndAbility))))))))))))

(event EventOnEndAbility
  (params (bWasCancelled :type Boolean))
  (Ability|RemoveGameplayEffectFromOwnerWithAssetTags "(GameplayTags=((TagName=\"skill.lazer.costEffect\")))")
  (Actor|DestroyActor (Variables|Default|GetLazerActor))
  (bind _bp_character_player (CallFunction|GetPlayerCharacterandController))
  (Default|SetUseControlRotatioinMode _bp_character_player true))