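; Projectile actor in the Fireball ability folder that delivers a Gameplay Effect to hostile characters it overlaps.
; On sphere overlap it checks hostility between the hit BP_CharacterBase and its instigator, then has the instigator apply the GESpecHandle variable to target data built from that actor.
; It destroys itself after a hostile hit, ignores other overlaps, and otherwise expires on a timer started at BeginPlay.
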(event OnComponentBeginOverlap(Sphere)
  (params (OverlappedComponent :type Primitive%20Component%20Object%20Reference) (OtherActor :type Actor%20Object%20Reference) (OtherComp :type Primitive%20Component%20Object%20Reference) (OtherBodyIndex :type Integer) (bFromSweep :type Boolean) (SweepResult :type Hit%20Result%20Structure%20%28by%20ref%29))
  (bind _returnvalue (Game|GetInstigator))
  (bind _asbp_character_base (Utilities|Casting|CastToBP_CharacterBase _returnvalue))
  (bind _asbp_character_base_2 (Utilities|Casting|CastToBP_CharacterBase OtherActor))
  (if (Class|QCharacterBase|IsHostile _asbp_character_base_2 _asbp_character_base)
    (Class|QCharacterBase|ApplyGESpecHandeltoTargetDataSpecHandle _asbp_character_base (Variables|Default|GetGESpecHandle) (Ability|TargetData|AbilityTargetDatafromActor OtherActor))
    (Actor|DestroyActor)))

(event Custom|AutoDestroyTimer
  (Actor|DestroyActor))

(event EventBeginPlay
  (Utilities|Time|SetTimerbyEvent (delegate Custom|AutoDestroyTimer) 6.0))

(event Collision|EventActorBeginOverlap
  (params (OtherActor :type Actor%20Object%20Reference)))

(event EventTick
  (params (DeltaSeconds :type Float%20%28single-precision%29)))

(fn ConstructionScript)