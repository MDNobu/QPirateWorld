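; Player Gameplay Ability for Ground Blast, a targeted attack that damages characters and launches them upward with a stun.
; After a resource check, it plays an intro montage, waits out its length, then uses a target data actor for user-confirmed targeting.
; Confirming commits the ability, starts cooldown and plays the cast montage while spawning the blast particle and applying the damage effect and push.
; It ends when targeting is cancelled or the cast montage finishes.
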(event Ability|EventActivateAbility
  (bind _costenough (CallFunction|IsCostResourceEnough))
  (if _costenough
    (|PlayMontageandWaitProxy "None" "/Game/_PirateWorld/Core/Characters/Animations/AM_Shinbi_GroundBlast.AM_Shinbi_GroundBlast" 1.0 "None" true 1.0 0.0
      (:then
        (Utilities|FlowControl|Delay (Variables|/Script/Engine.AnimSequenceBase|GetSequenceLength (Animation|GetCurrentMontage :!class /Script/GameplayAbilities.GameplayAbility)))
        (bind _data (|WaitTargetData :ConfirmationType "UserConfirmed" :Class "/Game/_PirateWorld/Core/Characters/GameplayAbilities/GroundBlast/BP_TargetDataActor_GroundBlast.BP_TargetDataActor_GroundBlast_C" :ReticleClass 0)
          (:ValidData
            (bind _bp_character_player (CallFunction|GetPlayerCharacterandController))
            (Variables|/Game/_PirateWorld/Core/Characters/BP_CharacterBase.BP_CharacterBase_C|SetbTargeting _bp_character_player false)
            (Ability|CommitAbility)
            (CallFunction|StartCooldown)
            (|PlayMontageandWaitProxy "None" "/Game/_PirateWorld/Core/Characters/Animations/AM_GroundBlast_Cast.AM_GroundBlast_Cast" 1.0 "None" true 1.0 0.0
              (:then
                (Effects|SpawnEmitteratLocation "/Game/_PirateWorld/Core/Characters/GameplayAbilities/GroundBlast/P_GroundBlast.P_GroundBlast" (Class|AbilitySystemBlueprintLibrary|GetTargetDataEndPoint _data (- (Ability|TargetData|GetDataCountfromTargetData _data) 1)))
                (GameplayEffects|ApplyGameplayEffectToTarget _data "/Game/_PirateWorld/Core/Characters/GameplayAbilities/GroundBlast/BP_GE_GroundBlast_DealDamage.BP_GE_GroundBlast_DealDamage_C" 1 1)
                (for _array_element (Ability|TargetData|GetActorsfromTargetData _data)
                  (bind _asbp_character_base (Utilities|Casting|CastToBP_CharacterBase _array_element))
                  (Default|PushandStunCharacter _asbp_character_base "0, 0,1.000000" 5e+02 2.0)))
              (:OnCompleted
                (Ability|EndAbility :!label _label))
              (:OnBlendOut
                (goto _label))
              (:OnInterrupted
                (goto _label))
              (:OnCancelled
                (goto _label))))
          (:Cancelled
            (Ability|EndAbility)))))))