(event Ability|EventActivateAbility
  (Ability|CommitAbility)
  (CallFunction|StartCooldown)
  (|PlayMontageandWaitProxy "None" "/Game/_PirateWorld/Core/Characters/Animations/AM_FireBlast.AM_FireBlast" 1.0 "None" true 1.0 0.0
    (:then
      (Ability|Tasks|WaitGameplayEvent "(TagName=\"skill.fireBlast.pull\")" 0
        (:EventReceived
          (bind _data (|WaitTargetData :ConfirmationType "Instant" :Class "/Script/QPirateWorld.QGATargetActor_FireBlast" :Radius 6e+02 :ReticleClass 0)
            (:then
              (Ability|Tasks|WaitGameplayEvent "(TagName=\"skill.fireBlast.push\")" 0
                (:EventReceived
                  (GameplayEffects|ApplyGameplayEffectToTarget (Variables|Default|GetTargetDataHandle) "/Game/_PirateWorld/Core/Characters/GameplayAbilities/FireBlast/BP_GE_FireBlast_DealDamage.BP_GE_FireBlast_DealDamage_C" 1 1)
                  (for _array_element (Ability|TargetData|GetActorsfromTargetData (Variables|Default|GetTargetDataHandle))
                    (bind _asbp_character_base (Utilities|Casting|CastToBP_CharacterBase _array_element))
                    (Default|PushandStunCharacter _asbp_character_base (Math|Vector|Normalize (- (Transformation|GetActorLocation _asbp_character_base) (Transformation|GetActorLocation (Ability|GetOwningActorfromActorInfo)))) 1e+03 3.0)))))
            (:ValidData
              (Variables|Default|SetTargetDataHandle _data)
              (for _array_element_2 (Ability|TargetData|GetActorsfromTargetData _data)
                (bind _asbp_character_base_2 (Utilities|Casting|CastToBP_CharacterBase _array_element_2))
                (Default|PushandStunCharacter _asbp_character_base_2 (Math|Vector|Normalize (- (Transformation|GetActorLocation (Ability|GetOwningActorfromActorInfo)) (Transformation|GetActorLocation _asbp_character_base_2))) 1e+03 3.0)))))))
    (:OnCompleted
      (Ability|EndAbility :!label _label))
    (:OnBlendOut
      (goto _label))
    (:OnInterrupted
      (goto _label))
    (:OnCancelled
      (goto _label))))

(event Ability|EventOnEndAbility
  (params (bWasCancelled :type Boolean)))