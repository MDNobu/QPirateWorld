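; Gameplay ability that dashes the player character forward, damaging, pushing and stunning characters it hits.
; On activation it commits, starts cooldown, zeroes ground friction, sets pawn collision to overlap, applies a forward impulse and plays the dash montage.
; A Skill.dash.dealDamage gameplay event supplies each target for the damage effect and a push away from the dasher.
; When the montage ends or is interrupted, it restores friction, blocks pawns again and ends.
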(event Ability|EventActivateAbility
  (Ability|CommitAbility)
  (CallFunction|StartCooldown)
  ;[1 1 1] Push forward Player character by Impulse
  (bind _bp_character_player (CallFunction|GetPlayerCharacterandController))
  (Utilities|IsValid _bp_character_player
    (:Is%20Valid
      (Variables|Default|SetOwningPlayerCharacter _bp_character_player)
      (Variables|Default|SetOriginalFriction (Variables|/Script/Engine.CharacterMovementComponent|GetGroundFriction (Variables|/Script/Engine.Character|GetCharacterMovement _bp_character_player)))
      (Variables|/Script/Engine.CharacterMovementComponent|SetGroundFriction (Variables|/Script/Engine.Character|GetCharacterMovement _bp_character_player) 0.0)
      (bind _bp_character_player_2 (CallFunction|GetPlayerCharacterandController))
      (Default|SetCollisionResponcetoPawn _bp_character_player_2 "ECR_Overlap")
      (Physics|AddImpulse (Variables|/Script/Engine.Character|GetCharacterMovement _bp_character_player) (* (Transformation|GetActorForwardVector _bp_character_player) 2e+05) false)
      ;[1 1 1] Play Dash Montage and End Ability when finished
      (|PlayMontageandWaitProxy "None" "/Game/_PirateWorld/Core/Characters/Animations/AM_Shinbi_Dash.AM_Shinbi_Dash" 1.0 "None" true 1.0 0.0
        (:then
          ;[1 1 1] Handle damage to other character and push back it
          (bind _payload (Ability|Tasks|WaitGameplayEvent "(TagName=\"skill.dash.dealDamage\")" 0)
            (:EventReceived
              (GameplayEffects|ApplyGameplayEffectToTarget (Ability|TargetData|AbilityTargetDatafromActor (.Target (Utilities|Struct|BreakGameplayEventData _payload))) "/Game/_PirateWorld/Core/Characters/GameplayAbilities/Dash/BP_GE_Dash_DealDamage.BP_GE_Dash_DealDamage_C" 1 1)
              (Default|PushandStunCharacter (.AsBP%20Character%20Base (Utilities|Casting|CastToBP_CharacterBase (.Target (Utilities|Struct|BreakGameplayEventData _payload)))) (Math|Vector|Normalize (- (Transformation|GetActorLocation (.AsBP%20Character%20Base (Utilities|Casting|CastToBP_CharacterBase (.Target (Utilities|Struct|BreakGameplayEventData _payload))))) (Transformation|GetActorLocation (Variables|Default|GetOwningPlayerCharacter)))) 2e+03 1e+01))))
        (:OnCompleted
          (Variables|/Script/Engine.CharacterMovementComponent|SetGroundFriction (Variables|/Script/Engine.Character|GetCharacterMovement (Variables|Default|GetOwningPlayerCharacter)) (Variables|Default|GetOriginalFriction) :!label _label)
          (Default|SetCollisionResponcetoPawn (Variables|Default|GetOwningPlayerCharacter) "ECR_Block")
          (Ability|EndAbility))
        (:OnBlendOut
          (goto _label))
        (:OnInterrupted
          (goto _label))
        (:OnCancelled
          (goto _label))))
    (:Is%20Not%20Valid
      (Ability|EndAbility))))

(event Ability|EventOnEndAbility
  (params (bWasCancelled :type Boolean)))