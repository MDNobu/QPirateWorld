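; BP_GA_Melee is a Gameplay Ability for a melee attack that plays the Shinbi melee montage.
; On activation it commits, starts the montage and waits for the deal-damage gameplay event.
; The event's target receives the melee damage effect, then is briefly stunned and pushed opposite its own forward vector, independent of the attacker's position.
; The ability ends when the montage completes, blends out, is interrupted or is cancelled.
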(event Ability|EventActivateAbility
  (Ability|CommitAbility)
  (|PlayMontageandWaitProxy "None" "/Game/_PirateWorld/Core/Characters/Animations/AM_Shinbi_Melee.AM_Shinbi_Melee" 1.0 "None" true 1.0 0.0
    (:then
      (bind _payload (Ability|Tasks|WaitGameplayEvent "(TagName=\"skill.melee.dealDamage\")" 0)
        (:EventReceived
          (GameplayEffects|ApplyGameplayEffectToTarget (Ability|TargetData|AbilityTargetDatafromActor (.Target (Utilities|Struct|BreakGameplayEventData _payload))) "/Game/_PirateWorld/Core/Characters/GameplayAbilities/Melee/BP_GE_Melee_DealDamage.BP_GE_Melee_DealDamage_C" 1 1)
          (Default|PushandStunCharacter (.AsBP%20Character%20Base (Utilities|Casting|CastToBP_CharacterBase (.Target (Utilities|Struct|BreakGameplayEventData _payload)))) (* (Transformation|GetActorForwardVector (.AsBP%20Character%20Base (Utilities|Casting|CastToBP_CharacterBase (.Target (Utilities|Struct|BreakGameplayEventData _payload))))) -1.0) 5e+01 0.3))))
    (:OnCompleted
      (Ability|EndAbility self :!label _label))
    (:OnBlendOut
      (goto _label))
    (:OnInterrupted
      (goto _label))
    (:OnCancelled
      (goto _label))))