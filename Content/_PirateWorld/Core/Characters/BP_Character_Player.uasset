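; Player character Blueprint that mirrors its attributes on the HUD's health, mana and strength balls.
; On possession it caches the BP_PlayerController, whose HUDWidget receives all updates.
; BeginPlay runs the parent logic, then fills only the health ball from HealthAttribute's current and max values.
; Health, mana and strength change events set the matching ball to the current-to-max ratio.
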(event EventBeginPlay
  (bind _healthattribute (Variables|Default|GetHealthAttribute))
  (|CallParentFunction)
  (Default|SetPercent (Variables|/Game/_PirateWorld/Core/UI/WBP_HUD.WBP_HUD_C|GetHealthBall (Variables|/Game/_PirateWorld/Core/PlayerController/BP_PlayerController.BP_PlayerController_C|GetHUDWidget (Variables|Default|GetBP%20Player%20Controller))) (/ (.currentvalue (Variables|/Script/QPirateWorld.QAttributeSetBase|GetHealth _healthattribute)) (.currentvalue (Variables|/Script/QPirateWorld.QAttributeSetBase|GetMaxHealth _healthattribute)))))

(event Collision|EventActorBeginOverlap
  (params (OtherActor :type Actor%20Object%20Reference))
  (|CallParentFunction OtherActor) ; This node is disabled and will not be called.\nDrag off pins to build functionality.
)

(event EventTick
  (params (DeltaSeconds :type Float%20%28single-precision%29)))

(event EventOnHealthChange
  (params (health :type Float%20%28single-precision%29) (maxHealth :type Float%20%28single-precision%29))
  (Default|SetPercent (Variables|/Game/_PirateWorld/Core/UI/WBP_HUD.WBP_HUD_C|GetHealthBall (Variables|/Game/_PirateWorld/Core/PlayerController/BP_PlayerController.BP_PlayerController_C|GetHUDWidget (Variables|Default|GetBP%20Player%20Controller))) (/ health maxHealth)))

(event EventOnManaChange
  (params (mana :type Float%20%28single-precision%29) (maxMana :type Float%20%28single-precision%29))
  (Default|SetPercent (Variables|/Game/_PirateWorld/Core/UI/WBP_HUD.WBP_HUD_C|GetManaBall (Variables|/Game/_PirateWorld/Core/PlayerController/BP_PlayerController.BP_PlayerController_C|GetHUDWidget (Variables|Default|GetBP%20Player%20Controller))) (/ mana maxMana)))

(event EventOnStrengthChange
  (params (strength :type Float%20%28single-precision%29) (maxStrength :type Float%20%28single-precision%29))
  (Default|SetPercent (Variables|/Game/_PirateWorld/Core/UI/WBP_HUD.WBP_HUD_C|GetStrengthBall (Variables|/Game/_PirateWorld/Core/PlayerController/BP_PlayerController.BP_PlayerController_C|GetHUDWidget (Variables|Default|GetBP%20Player%20Controller))) (/ strength maxStrength)))

(event EventPossessed
  (params (NewController :type Controller%20Object%20Reference))
  (bind _asbp_player_controller (Utilities|Casting|CastToBP_PlayerController NewController))
  (Variables|Default|SetBP%20Player%20Controller _asbp_player_controller))

(fn ConstructionScript
  (|CallParentFunction))