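; BP_Enemy is an enemy character Blueprint that displays its health through a health bar widget.
; On a health change event, it casts the HealthWidget component's user widget to WBP_HealthBar and sets the bar to current health divided by max health.
; The BeginPlay, overlap and Tick events are disabled placeholders, and the construction script only calls its parent.
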(event EventBeginPlay
  (|CallParentFunction) ; This node is disabled and will not be called.\nDrag off pins to build functionality.
)

(event Collision|EventActorBeginOverlap
  (params (OtherActor :type Actor%20Object%20Reference))
  (|CallParentFunction OtherActor) ; This node is disabled and will not be called.\nDrag off pins to build functionality.
)

(event EventTick
  (params (DeltaSeconds :type Float%20%28single-precision%29))
  (|CallParentFunction DeltaSeconds) ; This node is disabled and will not be called.\nDrag off pins to build functionality.
)

(event EventOnHealthChange
  (params (health :type Float%20%28single-precision%29) (maxHealth :type Float%20%28single-precision%29))
  (Default|SetHealthBarPercent (.AsWBP%20Health%20Bar (Utilities|Casting|CastToWBP_HealthBar (UserInterface|GetUserWidgetObject (Variables|Default|GetHealthWidget)))) (/ health maxHealth)))

(fn ConstructionScript
  (|CallParentFunction))