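; BP_CharacterBase is a character base for Pirate World that drives melee attacks through the Gameplay Ability System.
; It acquires BP_GA_Melee on BeginPlay, and PrimaryAttack activates that ability by class.
; When WeaponCollision overlaps another BP_Enemy-derived actor, it sends itself a Skill.melee.dealDamage gameplay event with that actor as target, leaving damage handling outside this Blueprint.
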(event OnComponentBeginOverlap(WeaponCollision)
  (params (OverlappedComponent :type Primitive%20Component%20Object%20Reference) (OtherActor :type Actor%20Object%20Reference) (OtherComp :type Primitive%20Component%20Object%20Reference) (OtherBodyIndex :type Integer) (bFromSweep :type Boolean) (SweepResult :type Hit%20Result%20Structure%20%28by%20ref%29))
  (if (and (!= OtherActor self) (Utilities|ClassIsChildOf (Utilities|GetClass OtherActor) "/Game/_PirateWorld/Core/Characters/BP_Enemy.BP_Enemy_C"))
    (Ability|SendGameplayEventtoActor self "(TagName=\"skill.melee.dealDamage\")" (Utilities|Struct|MakeGameplayEventData "(TagName=\"\")" 0 OtherActor))))

(event Custom|PrimaryAttack
  (Abilities|TryActivateAbilitybyClass (Variables|Default|GetAbilitySystemComp) "/Game/_PirateWorld/Core/Characters/GameplayAbilities/Melee/BP_GA_Melee.BP_GA_Melee_C" true))

(event EventBeginPlay
  (Class|QCharacterBase|AquireAbility "/Game/_PirateWorld/Core/Characters/GameplayAbilities/Melee/BP_GA_Melee.BP_GA_Melee_C"))

(event Collision|EventActorBeginOverlap
  (params (OtherActor :type Actor%20Object%20Reference)))

(fn ConstructionScript)